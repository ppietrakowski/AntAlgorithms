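; Game instance for an ant colony simulation that manages the UI and pheromone trail evaporation.
; On Init it creates the food adjustment and time widgets, with functions to show the former or swap it for the latter.
; Hiding food adjustment also starts a looping timer at the TimeScale interval.
; A separate update function applies the evaporation rate to every pheromone trail actor in the world.
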(event `self.ReceiveInit`
  (bind _returnvalue (`|CreateWidget` "/Game/Blueprints/Widgets/W_foodAdjustment.W_foodAdjustment_C"))
  (bind _returnvalue_2 (`|CreateWidget` "/Game/Blueprints/Widgets/W_time.W_time_C"))
  (set `self.W_FoodAdjustment` _returnvalue)
  (set `self.W_time` _returnvalue_2))

(fn `HideFoodAdjustment`
  (`Widget.RemoveFromParent` (`self.W_FoodAdjustment`))
  (`UserWidget.AddToViewport` (`self.W_time`) 0)
  (`self.StartEvaporating`))

(fn `ShowFoodAdjustment`
  (`UserWidget.AddToViewport` (`self.W_FoodAdjustment`) 0))

(fn `StartEvaporating`
  (`KismetSystemLibrary.K2_SetTimerDelegate` (`|CreateDelegate` :!event `UpdateEachTrail`) (`self.TimeScale`) true))

(fn `UpdateEachTrail`
  (bind _outactors (`GameplayStatics.GetAllActorsOfClass` "/Game/Blueprints/Actors/A_pheromoneTrail.A_pheromoneTrail_C"))
  (for _array_element _outactors
    (`/Game/Blueprints/Actors/A_pheromoneTrail.UpdatePheromone` _array_element (`/Game/Blueprints/GI_antColonySimulation.EvaporationRate` (cast `/Game/Blueprints/GI_antColonySimulation` (`GameplayStatics.GetGameInstance`) :!pure true)))))