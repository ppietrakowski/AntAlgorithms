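; StrenghtenTrail is a behaviour tree task that reinforces the trail an ant agent has stored in its blackboard.
; It sends the trail a strengthen message with the ant, its DistanceShortest value and a near-food flag set while NumTrails is still low.
; It then increments NumTrails and always finishes as failed.
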(event `self.ReceiveExecuteAI`
  (params (OwnerController :type "AIController Object Reference") (ControlledPawn :type "Pawn Object Reference"))
  (bind _numtrails (`self.NumTrails`))
  (bind _outant (message `/Game/Blueprints/Interfaces/IAnt.GetAsAnt` ControlledPawn))
  (message `/Game/Blueprints/Interfaces/Trail.Strenghten` (`BTFunctionLibrary.GetBlackboardValueAsObject` (`self.Trail`)) (<= (`BTFunctionLibrary.GetBlackboardValueAsInt` (`self.NumTrails`)) 2) _outant (`BTFunctionLibrary.GetBlackboardValueAsFloat` (`self.DistanceShortest`)))
  (`BTFunctionLibrary.SetBlackboardValueAsInt` _numtrails (+ (`BTFunctionLibrary.GetBlackboardValueAsInt` _numtrails) 1))
  (`self.FinishExecute` false))