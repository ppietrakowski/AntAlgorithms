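; Behavior tree task that pops the most recent trail from an ant pawn's TabuList, apparently for backtracking along visited trails.
; It removes the last entry and writes that trail actor and its location to the blackboard.
; An empty list clears HasTrail instead.
; Success and failure are inverted for selector flow: empty finishes as success to end the selector, while a successful pop finishes as failure so it continues.
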(event `self.ReceiveExecuteAI`
  (params (OwnerController :type "AIController Object Reference") (ControlledPawn :type "Pawn Object Reference"))
  (bind _outant (message `/Game/Blueprints/Interfaces/IAnt.GetAsAnt` ControlledPawn))
  (bind _tabulist (`/Game/Blueprints/Characters/C_ant.TabuList` _outant))
  (if (`KismetArrayLibrary.Array_IsEmpty` _tabulist)
    (`BTFunctionLibrary.SetBlackboardValueAsBool` (`self.HasTrail`))
    (`self.FinishExecute` true) ; Immediatelly ends selector :D
    (else
      (bind _returnvalue (`KismetArrayLibrary.Array_LastIndex` _tabulist))
      (bind _output_get (set `self.Trail` (`|GetArrayItem` _tabulist _returnvalue)))
      (`KismetArrayLibrary.Array_Remove` _tabulist _returnvalue)
      (`BTFunctionLibrary.SetBlackboardValueAsObject` (`self.OutTrail`) _output_get)
      (`BTFunctionLibrary.SetBlackboardValueAsVector` (`self.OutLocation`) (`Actor.K2_GetActorLocation` (`self.Trail`)))
      (`self.FinishExecute` false))))